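; BP_MyHero is the player character, handling camera-relative movement, look, selectable jump types, jogging and crouch input.
; JumpType picks a plain jump, a DoN-limited double jump using LaunchCharacter, or an unfinished third mode; landing resets the DoN.
; Jog raises walk speed, and its release sets a speed based on the crouch flag, which is all crouch input changes.
; BeginPlay randomizes NumberJumps, but the double jump overwrites it.
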(event EventOnLanded
  (params (Hit :type Hit%20Result%20Structure%20%28by%20ref%29))
  (Utilities|FlowControl|DoN (Variables|Default|GetNumberJumps)) ; enters at Reset
)

(event EventBeginPlay
  (Variables|Default|SetNumberJumps (Math|Random|RandomIntegerinRange 3 20)))

(event Input|ActionEvents|InputActionJump
  (params (Key :type Key%20Structure :default "None"))
  (:Pressed
    (switch int (Variables|Default|GetJumpType)
      (:0
        (Character|Jump))
      (:1
        (Variables|Default|SetNumberJumps 2)
        (bind _counter (Utilities|FlowControl|DoN (Variables|Default|GetNumberJumps) :!label _label)
          (:Exit
            (if (and (>= _counter 2) (<= _counter (Variables|Default|GetNumberJumps)))
              (bind _output_get (Variables|Default|SetCounter 2)))
            (switch int _output_get
              (:1
                (Character|Jump))
              (:2
                (Character|LaunchCharacter (Math|Vector|MakeVector 0.0 0.0 (Variables|/Script/Engine.CharacterMovementComponent|GetJumpZVelocity (Variables|Character|GetCharacterMovement))) false false) ; El vector amarillo cambio a component, click secundario split struct pin sobre el nodo amarillo original
                (Development|PrintString (Utilities|String|ToString(Integer) (Variables|Default|GetNumberJumps))))))))
      (:2
        (goto _label)))))

(event Input|ActionEvents|InputActionJog
  (params (Key :type Key%20Structure :default "None"))
  (bind _charactermovement (Variables|Character|GetCharacterMovement))
  (:Pressed
    (Variables|Actor|SetJogPressed true)
    (Variables|/Script/Engine.CharacterMovementComponent|SetMaxWalkSpeed _charactermovement (+ (Variables|/Script/Engine.CharacterMovementComponent|GetMaxWalkSpeed _charactermovement) 2e+02)))
  (:Released
    (Variables|Actor|SetJogPressed false)
    (if (Variables|Actor|GetCrouchPressed)
      (bind _output_get (Variables|/Script/Engine.CharacterMovementComponent|SetMaxWalkSpeed _charactermovement 4e+02))
      (Development|PrintString (Utilities|String|ToString(Float) _output_get))
      (else
        (Variables|/Script/Engine.CharacterMovementComponent|SetMaxWalkSpeed _charactermovement 6e+02)))))

(event Input|ActionEvents|InputActionCrouch
  (params (Key :type Key%20Structure :default "None"))
  (:Pressed
    (Variables|Actor|SetCrouchPressed true))
  (:Released
    (Variables|Actor|SetCrouchPressed false)))

(event Input|AxisEvents|InputAxisMove_X
  (params (AxisValue :type Float%20%28single-precision%29))
  (Pawn|Input|AddMovementInput (Math|Vector|GetRightVector (Math|Rotator|MakeRotator 0.0 0.0 (.Yaw (Math|Rotator|BreakRotator (Pawn|GetControlRotation :!class /Script/Engine.Pawn))))) AxisValue false))

(event Input|AxisEvents|InputAxisMove_Y
  (params (AxisValue :type Float%20%28single-precision%29))
  (Pawn|Input|AddMovementInput (Math|Vector|GetForwardVector (Math|Rotator|MakeRotator 0.0 0.0 (.Yaw (Math|Rotator|BreakRotator (Pawn|GetControlRotation :!class /Script/Engine.Pawn))))) AxisValue false))

(event Input|AxisEvents|InputAxisTurn
  (params (AxisValue :type Float%20%28single-precision%29))
  (Pawn|Input|AddControllerYawInput AxisValue))

(event Input|AxisEvents|InputAxisLockUp
  (params (AxisValue :type Float%20%28single-precision%29))
  ;[1 1 1] Go into your Camera component. In the Details panel search for 'Use Pawn Control Rotation' and make sure that it is enabled
  (Pawn|Input|AddControllerPitchInput AxisValue))

(fn ConstructionScript)